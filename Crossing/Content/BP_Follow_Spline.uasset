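; BP_Follow_Spline is an actor that moves a cube along its spline component at a set speed.
; Each tick it advances a distance counter by speed times delta time and snaps the cube's world transform to that point on the spline, ignoring scale.
; When looping is enabled, the distance resets to zero once it reaches the spline's length.
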(event EventTick
  (params (DeltaSeconds :type Float%20%28single-precision%29))
  (bind _output_get (Variables|Default|SetPosition_on_Spline (+ (* DeltaSeconds (Variables|Default|GetSpeed_on_Spline)) (Variables|Default|GetPosition_on_Spline))))
  (Transformation|SetWorldTransform (Variables|Default|GetCube) (Spline|GetTransformatDistanceAlongSpline (Variables|Default|GetSpline) _output_get "World" false) false false)
  (if (Variables|Default|GetLoop)
    (if (>= (Variables|Default|GetPosition_on_Spline) (Spline|GetSplineLength (Variables|Default|GetSpline)))
      (Variables|Default|SetPosition_on_Spline 0.0))))

(fn ConstructionScript)